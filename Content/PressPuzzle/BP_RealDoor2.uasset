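; Door actor for the press puzzle that slides its static mesh along the Z axis when opened.
; OpenDoors enables actor tick, and each Tick plays a timeline whose track sets the mesh's relative Z while keeping X and Y.
; Tick is never switched off in live logic: the shutoff check, rotation timeline and location lerp are disconnected leftovers, so the values cached at BeginPlay go unused.
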(event EventOpenDoors
  (Actor|Tick|SetActorTickEnabled true))

(event EventTick
  (params (DeltaSeconds :type Float%20%28single-precision%29))
  (bind _staticmesh (Variables|Default|GetStaticMesh))
  (bind _relativelocation (Variables|/Script/Engine.SceneComponent|GetRelativeLocation _staticmesh))
  (Variables|Default|SetCurrentTime (+ DeltaSeconds (Variables|Default|GetCurrentTime)))
  (bind _newtrack_0 (Timeline|Timeline_0 Play)
    (:Update
      (Transformation|SetRelativeLocation _staticmesh (Math|Vector|MakeVector (.x _relativelocation) (.y _relativelocation) (.z _newtrack_0)) false false))))

(event EventBeginPlay
  (Variables|Default|SetStartLocation (Transformation|GetActorLocation))
  (Variables|Default|SetDefaultRotator (Transformation|GetWorldRotation (Variables|Default|GetDefaultSceneRoot))))

(fn ConstructionScript)