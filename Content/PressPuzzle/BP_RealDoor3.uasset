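; Door for the nine-square press puzzle that moves its mesh vertically once the puzzle is solved.
; A looping half-second timer polls every BP_NinePuzzle actor, counting cubes whose material is the lit square instance.
; A count of nine plays a timeline driving the mesh's relative Z; the timer keeps running and printing debug output.
; OpenDoors only enables a time-accumulating Tick, as the older rotate and lerp logic is disconnected.
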(event Custom|UpNineDoor
  (bind _staticmesh (Variables|Default|GetStaticMesh))
  (bind _relativelocation (Variables|/Script/Engine.SceneComponent|GetRelativeLocation _staticmesh))
  (bind _newtrack_0 (Timeline|Timeline_0 Play)
    (:Update
      (Transformation|SetRelativeLocation _staticmesh (Math|Vector|MakeVector (.x _relativelocation) (.y _relativelocation) (.z _newtrack_0)) false false))))

(event EventOpenDoors
  (Actor|Tick|SetActorTickEnabled true))

(event EventTick
  (params (DeltaSeconds :type Float%20%28single-precision%29))
  (Variables|Default|SetCurrentTime (+ DeltaSeconds (Variables|Default|GetCurrentTime))))

(event EventBeginPlay
  (Variables|Default|SetStartLocation (Transformation|GetActorLocation))
  (Variables|Default|SetDefaultRotator (Transformation|GetWorldRotation (Variables|Default|GetDefaultSceneRoot)))
  (Utilities|Time|SetTimerbyFunctionName 0 "CheckMaterial" 0.5 true))

(fn ConstructionScript)

(fn CheckMaterial
  (Development|PrintString "Call CheckMaterial")
  (bind _outactors (Actor|GetAllActorsOfClass "/Game/NinePuzzle/BP_NinePuzzle.BP_NinePuzzle_C"))
  (Development|PrintString (Utilities|String|ToString(Integer) (Utilities|Array|Length _outactors)))
  (for _array_element _outactors
    (Development|PrintText (Utilities|Text|ToText(Object) (Rendering|Material|GetMaterial (Variables|/Game/NinePuzzle/BP_NinePuzzle.BP_NinePuzzle_C|GetCube _array_element) 0)))
    (if (== (Rendering|Material|GetMaterial (Variables|/Game/NinePuzzle/BP_NinePuzzle.BP_NinePuzzle_C|GetCube _array_element) 0) "/Game/AssetPacks/ModularSciFiSeason1/StarterBundle/ModularScifiHallways/Materials/MI_Hall_Light_Square_M.MI_Hall_Light_Square_M")
      (Variables|Default|SetCorrectNum (+ (Variables|Default|GetCorrectNum) 1.0))
      (if (== (Variables|Default|GetCorrectNum) 9.0)
        (CallFunction|UpNineDoor)
        (Variables|Default|SetCorrectNum 0.0))))
  (Variables|Default|SetCorrectNum 0.0))