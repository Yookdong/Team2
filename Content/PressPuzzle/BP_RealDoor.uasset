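; Door actor, in the PressPuzzle folder, that moves its static mesh along a Timeline track when OpenDoors is called.
; OpenDoors enables actor Tick, which accumulates elapsed time and calls Play on the Timeline to drive the mesh's relative location.
; Timeline updates switch Tick off once elapsed time reaches RotationTime.
; BeginPlay caches start location and rotation, used only by disconnected leftover lerp and rotation nodes.
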(event EventOpenDoors
  (Actor|Tick|SetActorTickEnabled true))

(event EventTick
  (params (DeltaSeconds :type Float%20%28single-precision%29))
  (Variables|Default|SetCurrentTime (+ DeltaSeconds (Variables|Default|GetCurrentTime)))
  (bind _newtrack_0 (Timeline|Timeline Play)
    (:Update
      (Transformation|SetRelativeLocation (Variables|Default|GetStaticMesh) _newtrack_0 false false)
      (if (>= (Variables|Default|GetCurrentTime) (Variables|Default|GetRotationTime))
        (Actor|Tick|SetActorTickEnabled false)))))

(event EventBeginPlay
  (Variables|Default|SetStartLocation (Transformation|GetActorLocation))
  (Variables|Default|SetDefaultRotator (Transformation|GetWorldRotation (Variables|Default|GetDefaultSceneRoot))))

(fn ConstructionScript)