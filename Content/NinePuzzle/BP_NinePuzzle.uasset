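; BP_NinePuzzle is a pad in a Lights Out-style puzzle, where stepping on one toggles it and its linked pads.
; Overlap by a BP_TPBaseCharacter flips IsAttached on itself and on every pad in its AttachPad array.
; Tick swaps the cube between two hall light materials from that flag, and OpenDoors only enables ticking.
; CheckMaterial loops over all pads comparing materials to IsOn but does nothing with the result.
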(event EventOpenDoors
  (Actor|Tick|SetActorTickEnabled true))

(event Collision|EventActorBeginOverlap
  (params (OtherActor :type Actor%20Object%20Reference))
  (if (== (Utilities|GetClass OtherActor) "/Game/TeamProject/GameMode/BP_TPBaseCharacter.BP_TPBaseCharacter_C")
    (if (Variables|Default|GetIsAttached)
      (Variables|Default|SetIsAttached false)
      (else
        (Variables|Default|SetIsAttached true)))
    (for _array_element (Variables|Default|GetAttachPad)
      (if (Variables|BP_NinePuzzle_C|GetIsAttached _array_element)
        (Variables|BP_NinePuzzle_C|SetIsAttached _array_element false)
        (else
          (Variables|BP_NinePuzzle_C|SetIsAttached _array_element true))))))

(event EventTick
  (params (DeltaSeconds :type Float%20%28single-precision%29))
  (bind _cube (Variables|Default|GetCube))
  (if (Variables|Default|GetIsAttached)
    (Rendering|Material|SetMaterial _cube 0 "/Game/AssetPacks/ModularSciFiSeason1/StarterBundle/ModularScifiHallways/Materials/MI_Hall_Light_Square_M.MI_Hall_Light_Square_M")
    (else
      (Rendering|Material|SetMaterial _cube 0 "/Game/AssetPacks/ModularSciFiSeason1/StarterBundle/ModularScifiHallways/Materials/MI_Hall_Light_Square_M_2.MI_Hall_Light_Square_M_2"))))

(fn ConstructionScript)

(fn CheckMaterial
  (bind _outactors (Actor|GetAllActorsOfClass "BP_NinePuzzle_C"))
  (for _array_element _outactors
    (if (== (Rendering|Material|GetMaterial (Variables|Default|GetCube) 0) "/Game/NinePuzzle/IsOn.IsOn")
      _)))