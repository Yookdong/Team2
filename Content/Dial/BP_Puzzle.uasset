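; BP_Puzzle is a three-dial combination lock that opens a linked door when every dial matches its code.
; InteractwithPuzzle rolls the passed dial left or right by RotateValue and prints its rotation.
; CheckCode then compares that dial's relative roll to its Code entry within a small tolerance and stores the result in AvailableCode.
; The door opens if all stored results are true and closes otherwise.
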(event EventInteractwithPuzzle
  (params (Component :type Primitive%20Component%20Object%20Reference) (RotateLeft :type Boolean))
  (CallFunction|Rotate Component RotateLeft))

(fn ConstructionScript)

(fn Rotate
  (params (Component :type Primitive%20Component%20Object%20Reference) (RotateLeft :type Boolean))
  (if RotateLeft
    (Transformation|AddRelativeRotation Component (Math|Rotator|MakeRotator (* (Variables|Default|GetRotateValue) 1.0) 0.0 0.0) false false)
    (else
      (Transformation|AddRelativeRotation Component (Math|Rotator|MakeRotator (* (Variables|Default|GetRotateValue) -1.0) 0.0 0.0) false false)))
  (Development|PrintString (Utilities|String|ToString(Rotator) (Variables|/Script/Engine.SceneComponent|GetRelativeRotation Component)))
  (CallFunction|CheckCode Component))

(fn CheckCode
  (params (Component :type Primitive%20Component%20Object%20Reference))
  (bind _door (Variables|Default|GetDoor))
  (if (== Component (Variables|Default|GetFirstDial))
    (LocalVariables|SetSelectedMesh 0)
    (Utilities|Array|SetArrayElem (Variables|Default|GetAvailableCode) (LocalVariables|GetSelectedMesh) (Math|Float|NearlyEqual(Float) (Utilities|Array|Get(acopy) (Variables|Default|GetCode) (LocalVariables|GetSelectedMesh)) (.roll (Variables|/Script/Engine.SceneComponent|GetRelativeRotation Component)) 1.0) :!label _label)
    (bind _array_element (Utilities|Array|ForEachLoopwithBreak (Variables|Default|GetAvailableCode) :!label _label_2)
      (:LoopBody
        (if (not _array_element)
          (LocalVariables|SetLocalFailed true)
          (goto _label_2 Break)))
      (:Completed
        (if (LocalVariables|GetLocalFailed)
          (Default|CloseDoor _door)
          (else
            (Default|OpenDoor _door)))))
    (elif (== Component (Variables|Default|GetSecondDial))
      (LocalVariables|SetSelectedMesh 1)
      (goto _label)
      (elif (== Component (Variables|Default|GetThirdDial))
        (LocalVariables|SetSelectedMesh 2)
        (goto _label)))))