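; Door Blueprint in the Dial folder that slides its static mesh vertically to open and close.
; ReqOpen calls ResOpen, which calls OpenDoorDial; the OpenDoor_Dial event calls OpenDoor and plays DoorTimeline.
; The timeline drives only the mesh's relative Z, keeping X and Y, and CloseDoor reverses it.
; A rotator combine with DefaultRotation is left unused.
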(event Custom|OpenDoor_Dial
  (bind _staticmesh (Variables|Default|GetStaticMesh))
  (bind _relativelocation (Variables|/Script/Engine.SceneComponent|GetRelativeLocation _staticmesh))
  (Class|MissionController|OpenDoor)
  (bind _newtrack_0 (Timeline|DoorTimeline Play)
    (:Update
      (Transformation|SetRelativeLocation _staticmesh (Math|Vector|MakeVector (.x _relativelocation) (.y _relativelocation) (.z _newtrack_0)) false false))))

(event Custom|CloseDoor
  (bind _staticmesh (Variables|Default|GetStaticMesh))
  (bind _relativelocation (Variables|/Script/Engine.SceneComponent|GetRelativeLocation _staticmesh))
  (bind _newtrack_0 (Timeline|DoorTimeline Reverse)
    (:Update
      (Transformation|SetRelativeLocation _staticmesh (Math|Vector|MakeVector (.x _relativelocation) (.y _relativelocation) (.z _newtrack_0)) false false))))

(event Custom|ReqOpen
  (CallFunction|ResOpen))

(event Custom|ResOpen
  (CallFunction|OpenDoorDial))

(fn ConstructionScript)