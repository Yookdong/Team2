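; Laser emitter actor that casts a reflecting beam from its arrow to activate sensors and open a door.
; On Tick, after a short delay, CastLight destroys old beams, switches off the stored sensor and re-traces the path.
; ArrowMaterial faces mirror the ray, while M_Glass faces activate the hit actor and message the door.
; Face materials identify surfaces, and each segment spawns a LaserBeam actor.
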(event EventTick
  (params (DeltaSeconds :type Float%20%28single-precision%29))
  (bind _arrow (Variables|Default|GetArrow))
  (Utilities|FlowControl|Delay 0.01)
  (CallFunction|CastLight (Transformation|GetWorldLocation _arrow) (Math|Vector|GetForwardVector _arrow) (Variables|Default|GetCastDistance)))

(fn ConstructionScript)

(fn CastLight
  (params (CastOrigin :type Vector) (Cast%20Direction :type Vector) (Cast%20Distance :type Float%20%28double-precision%29))
  (LocalVariables|SetL_CastOrigin CastOrigin)
  (LocalVariables|SetL_CastDirection Cast%20Direction)
  (LocalVariables|SetL_CastDistance Cast%20Distance)
  (for _array_element (Variables|Default|GetBeams)
    (Actor|DestroyActor _array_element))
  (Utilities|Array|Clear (Variables|Default|GetBeams))
  (Class|BPISetState|ToggleState(Message) (Variables|Default|GetActivatedSensor) false)
  (while (LocalVariables|GetL_Continue)
    (Utilities|FlowControl|Sequence
      (:then_0
        (bind (_outhit _returnvalue) (Collision|LineTraceByChannel (LocalVariables|GetL_CastOrigin) (+ (LocalVariables|GetL_CastOrigin) (* (LocalVariables|GetL_CastDirection) (LocalVariables|GetL_CastDistance))) "TraceTypeQuery3" true 0 "ForDuration" true "(R=1.000000,G=0.000000,B=0.000000,A=1.000000)" "(R=0.000000,G=1.000000,B=0.000000,A=1.000000)" 0.1))
        (LocalVariables|SetL_BeamStart (LocalVariables|GetL_CastOrigin))
        (if _returnvalue
          (LocalVariables|SetL_BeamEnd (.ImpactPoint (Collision|BreakHitResult _outhit)))
          (if (== (.ReturnValue (Class|PrimitiveComponent|GetMaterialfromCollisionFaceIndex (.HitComponent (Collision|BreakHitResult _outhit)) (.FaceIndex (Collision|BreakHitResult _outhit)))) "/Engine/VREditor/UI/ArrowMaterial.ArrowMaterial")
            (LocalVariables|SetL_CastOrigin (.ImpactPoint (Collision|BreakHitResult _outhit)))
            (LocalVariables|SetL_CastDirection (Math|Vector|MirrorVectorbyNormal (LocalVariables|GetL_CastDirection) (.ImpactNormal (Collision|BreakHitResult _outhit))))
            (LocalVariables|SetL_Continue true)
            (else
              (if (== (.ReturnValue (Class|PrimitiveComponent|GetMaterialfromCollisionFaceIndex (.HitComponent (Collision|BreakHitResult _outhit)) (.FaceIndex (Collision|BreakHitResult _outhit)))) "/Game/StarterContent/Materials/M_Glass.M_Glass")
                (Class|BPISetState|ToggleState(Message) (.HitActor (Collision|BreakHitResult _outhit)) true)
                (Variables|Default|SetActivatedSensor (.HitActor (Collision|BreakHitResult _outhit)))
                (Class|PuzzleInterface|OpenDoors(Message) (Variables|Default|GetDoor)))
              (LocalVariables|SetL_Continue false :!label _label)))
          (else
            (LocalVariables|SetL_BeamEnd (+ (LocalVariables|GetL_CastOrigin) (* (LocalVariables|GetL_CastDirection) (LocalVariables|GetL_CastDistance))))
            (goto _label))))
      (:then_1
        (bind _returnvalue_2 (Game|SpawnActorfromClass "/Game/Laser/Blueprint/LaserBeam.LaserBeam_C" (Math|Transform|MakeTransform "0, 0, 0" "0, 0, 0" "1.000000,1.000000,1.000000") "Undefined" "MultiplyWithRoot" 0 0))
        (Default|SetEnds _returnvalue_2 (LocalVariables|GetL_BeamStart) (LocalVariables|GetL_BeamEnd))
        (Utilities|Array|Add (Variables|Default|GetBeams) _returnvalue_2)))))