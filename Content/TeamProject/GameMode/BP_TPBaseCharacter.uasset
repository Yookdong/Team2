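; Base multiplayer player character with a flashlight that damages monsters and input for rotating puzzles.
; Left mouse toggles the light via server-to-multicast events; monster overlap starts a looping point-damage timer while it is on.
; Q/E line-trace forward and message the hit puzzle with a rotation direction.
; Incoming damage lowers PlayerState HP with brief invulnerability, while Tick stores authority-side control rotation and snaps the local ragdolled actor to its spine.
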(event OnComponentBeginOverlap(LightActor)
  (params (OverlappedComponent :type Primitive%20Component%20Object%20Reference) (OtherActor :type Actor%20Object%20Reference) (OtherComp :type Primitive%20Component%20Object%20Reference) (OtherBodyIndex :type Integer) (bFromSweep :type Boolean) (SweepResult :type Hit%20Result%20Structure%20%28by%20ref%29))
  (if (Variables|Light|GetIsCanDamage?)
    (for _array_element (Collision|GetOverlappingActors (Variables|Default|GetLightActor) "/Game/BG/BP/AI/BP_Monster.BP_Monster_C" :!class /Script/Engine.PrimitiveComponent)
      (bind _returnvalue (Utilities|Time|SetTimerbyFunctionName 0 "GetMonsterDamage" 0.3 true)))))

(event OnComponentEndOverlap(LightActor)
  (params (OverlappedComponent :type Primitive%20Component%20Object%20Reference) (OtherActor :type Actor%20Object%20Reference) (OtherComp :type Primitive%20Component%20Object%20Reference) (OtherBodyIndex :type Integer))
  (Utilities|Time|ClearandInvalidateTimerbyHandle (stale OnComponentBeginOverlap(LightActor) _returnvalue)))

(event Custom|LightOnServer
  (CallFunction|LightonMulticast))

(event Custom|LightOnMulticast
  (if (Variables|Light|GetIsCanDamage?)
    (Development|SetHiddeninGame (Variables|Default|GetSpotLight) true false)
    (Variables|Light|SetIsCanDamage? false)
    (else
      (Development|SetHiddeninGame (Variables|Default|GetSpotLight) false false)
      (Variables|Light|SetIsCanDamage? true))))

(event EventTick
  (params (DeltaSeconds :type Float%20%28single-precision%29))
  (Utilities|FlowControl|Sequence
    (:then_0
      (Networking|SwitchHasAuthority
        (:Authority
          (Variables|Character|SetPlayerRotation (Pawn|GetControlRotation :!class /Script/Engine.Pawn)))))
    (:then_1
      (if (Variables|캐릭터|GetIsRagdoll?)
        (if (== (Game|GetPlayerCharacter 0) self)
          (Transformation|SetActorLocation (Transformation|GetSocketLocation (Variables|Character|GetMesh) "spine_02") false false))))))

(event Game|Damage|EventAnyDamage
  (params (Damage :type Float%20%28single-precision%29) (DamageType :type Damage%20Type%20Object%20Reference) (InstigatedBy :type Controller%20Object%20Reference) (DamageCauser :type Actor%20Object%20Reference))
  (Camera|PlayWorldCameraShake "/Game/BG/BP/Camera/Shake_Attack.Shake_Attack_C" "0, 0, 0" 0.0 1e+03)
  (bind _asbp_tpplayer_state (Utilities|Casting|CastToBP_TPPlayerState (Variables|Default|GetPlayerState)))
  (Variables|/Script/TeamProject.TPPlayerState|SetCurrentHP _asbp_tpplayer_state (Variables|/Script/TeamProject.TPPlayerState|GetCurrentHP _asbp_tpplayer_state))
  (if (Variables|캐릭터|GetIsDamage?)
    (bind _output_get (Variables|/Script/TeamProject.TPPlayerState|SetCurrentHP _asbp_tpplayer_state (- (Variables|/Script/TeamProject.TPPlayerState|GetCurrentHP _asbp_tpplayer_state) Damage)))
    (if (<= _output_get 0.0)
      ;[1 0.05157 0] + 죽음 처리
      (Actor|DestroyActor)
      (else
        (Variables|캐릭터|SetIsDamage? false)
        (Utilities|FlowControl|Delay 0.5)
        (Variables|캐릭터|SetIsDamage? true)))))

(event Input|KeyboardEvents|E
  (params (Key :type Key%20Structure))
  (:Pressed
    (Variables|Default|SetRotateLeft false)
    (CallFunction|InteractwithPuzzle)))

(event Input|KeyboardEvents|Q
  (params (Key :type Key%20Structure))
  (:Pressed
    (Variables|Default|SetRotateLeft true)
    (CallFunction|InteractwithPuzzle)))

(event Input|MouseEvents|LeftMouseButton
  (params (Key :type Key%20Structure))
  (:Pressed
    (if (not (Variables|캐릭터|GetIsRagdoll?))
      (CallFunction|LightonServer))))

(fn ConstructionScript)

(fn GetMonsterDamage
  (for _array_element (Collision|GetOverlappingActors (Variables|Default|GetLightActor) "/Game/BG/BP/AI/BP_Monster.BP_Monster_C" :!class /Script/Engine.PrimitiveComponent)
    (Game|Damage|ApplyPointDamage _array_element 1e+01 (Transformation|GetActorLocation _array_element) (Collision|MakeHitResult false false 0.0 0.0 "0, 0, 0" "0, 0, 0" "0,0,1" "0,0,1" 0 _array_element) 0 self)))

(fn IsEquipB
  (return true))

(fn GetMultiPlayerRotation
  (if (== (Game|GetPlayerCharacter 0) self)
    (return (Pawn|GetControlRotation :!class /Script/Engine.Pawn))
    (else
      (return (Variables|Character|GetPlayerRotation)))))

(fn InteractwithPuzzle
  (bind _capsulecomponent (Variables|Default|GetCapsuleComponent))
  (bind _returnvalue (Transformation|GetWorldLocation _capsulecomponent))
  (bind (_outhit _returnvalue_2) (Collision|LineTraceByChannel _returnvalue (+ _returnvalue (* (Math|Vector|GetForwardVector _capsulecomponent) 4e+02)) "TraceTypeQuery1" false 0 "None"))
  (if _returnvalue_2
    (Class|InteractwithPuzzle|InteractwithPuzzle(Message) (.HitActor (Collision|BreakHitResult _outhit)) (.HitComponent (Collision|BreakHitResult _outhit)) (Variables|Default|GetRotateLeft))))