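; BP_Weapon is a light item that the player picks up by walking into it.
; On sphere overlap it unhides the player's own BPWeapon component, sets HaveLight and destroys itself.
; OnLightProjectile's condition is fixed true, so it only clears the light flags; a multicast event plays sounds at a location.
; Owner-based pickup and drop helpers remain, but the socket attach and anim-instance setup is unreachable.
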(event OnComponentBeginOverlap(SphereCollision)
  (params (OverlappedComponent :type Primitive%20Component%20Object%20Reference) (OtherActor :type Actor%20Object%20Reference) (OtherComp :type Primitive%20Component%20Object%20Reference) (OtherBodyIndex :type Integer) (bFromSweep :type Boolean) (SweepResult :type Hit%20Result%20Structure%20%28by%20ref%29))
  (bind _asbp_test_player (Utilities|Casting|CastToBP_TestPlayer OtherActor))
  (Development|SetHiddeninGame (Variables|/Game/BG/BP/BP_TestPlayer.BP_TestPlayer_C|GetBP_Weapon _asbp_test_player) false false)
  (Variables|/Game/BG/BP/BP_TestPlayer.BP_TestPlayer_C|SetHaveLight? _asbp_test_player true)
  (Actor|DestroyActor))

(event Custom|Play%20Sound%20Multicast
  (params (Sound :type Sound%20Base%20Object%20Reference) (Location :type Vector))
  (Audio|PlaySoundatLocation Sound Location "0, 0, 0" 1.0 1.0 0.0 0 0 0 0) ; Play firing sound
)

(event Custom|OnLightProjectile
  (bind _ownchar (Variables|Default|GetOwnChar))
  (if true
    (Variables|Default|SetIsClickLight? false)
    (Variables|Default|SetIsActorOn? false)
    (Variables|/Game/BG/BP/BP_TestPlayer.BP_TestPlayer_C|SetIsOnLight? _ownchar false)
    (else
      (Variables|Default|SetIsClickLight? true)
      (Variables|Default|SetIsActorOn? true)
      (Variables|/Game/BG/BP/BP_TestPlayer.BP_TestPlayer_C|SetIsOnLight? _ownchar true))))

(fn ConstructionScript)

(fn EventDrop
  (params (Character :type Character%20Object%20Reference))
  (Variables|Default|SetOwnChar 0))

(fn IsCanPickUp
  (Utilities|IsValid (Variables|Default|GetOwnChar)
    (:Is%20Valid
      (return false))
    (:Is%20Not%20Valid
      (return true))))