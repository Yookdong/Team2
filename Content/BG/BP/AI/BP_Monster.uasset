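; AI monster character that hunts the player, deals melee damage and plays a looping background sound.
; Sight and hearing perception write target and status to the Blackboard, with a cooldown on hearing.
; Overlaps on an attack sphere damage the target during attacks, gated by a resettable DoOnce.
; Incoming damage updates health and can trigger fleeing, but zero health only makes it unbeatable because the death logic is disconnected.
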(event OnTargetPerceptionUpdated(Monster_AIPerception)
  (params (Actor :type Actor%20Object%20Reference) (Stimulus :type AI%20Stimulus%20Structure))
  (CallFunction|MonsterPerception Actor Stimulus))

(event OnComponentBeginOverlap(Sphere_r)
  (params (OverlappedComponent :type Primitive%20Component%20Object%20Reference) (OtherActor :type Actor%20Object%20Reference) (OtherComp :type Primitive%20Component%20Object%20Reference) (OtherBodyIndex :type Integer) (bFromSweep :type Boolean) (SweepResult :type Hit%20Result%20Structure%20%28by%20ref%29))
  (bind _returnvalue (AI|GetBlackboard 0))
  ;[1 1 1] Player Damage
  (if (Variables|Default|GetIsOnAttack?)
    (Utilities|IsValid _returnvalue
      (:Is%20Valid
        (if (and (== OtherActor (AI|Components|Blackboard|GetValueasObject _returnvalue (Utilities|Name|MakeLiteralName "TargetActor"))) (Variables|Default|GetCanApplyDamage?))
          (Utilities|FlowControl|DoOnce false
            (:Completed
              (Game|Damage|ApplyDamage OtherActor (Variables|MonsterValues|GetBase%20Damage) 0 self))))))))

(event Custom|InitiateMonsterAI
  (AI|Components|Blackboard|SetValueasBool (AI|GetBlackboard 0) (Utilities|Name|MakeLiteralName "PatrolLooping?") (Variables|Monster|GetPatrolLooping?))
  (AI|Components|Blackboard|SetValueasEnum (AI|GetBlackboard 0) (Utilities|Name|MakeLiteralName "InitialState") (Variables|Monster|GetInitialState))
  (Variables|Default|SetSpawnPoint (Transformation|GetActorLocation)))

(event Custom|DestroyAIMulticast
  (Components|DestroyComponent (Variables|Default|GetMonster_AIPerception))
  (Utilities|IsValid (Pawn|GetController)
    (:Is%20Valid
      (Pawn|UnPossess (Pawn|GetController))
      (Components|DestroyComponent (Variables|Collision|GetCapsuleComponent))
      (Collision|SetCollisionProfileName (Variables|Character|GetMesh) "Ragdoll" true :!class /Script/Engine.PrimitiveComponent)
      (Pawn|Components|CharacterMovement|SetMovementMode (Variables|Character|GetCharacterMovement) "MOVE_None" 0))))

(event Custom|Monster_OnInvestigateEachRound)

(event Custom|Monster_OnHearing)

(event Custom|ResetHearing
  (Utilities|FlowControl|Delay 2.0)
  (Variables|Default|SetCanSearch? true))

(event Custom|Monster_OnAttackStart
  (Variables|Default|SetIsOnAttack? true))

(event Custom|Monster_OnAttackFinished
  (Variables|Default|SetIsOnAttack? false))

(event Custom|PlayEmitterMulticast
  (Effects|SpawnEmitterAttached (Variables|Monster|GetDamageEffect) (Variables|Character|GetMesh) "None" (+ (+ (Transformation|GetActorLocation) "0.000000,0.000000,120.000000") (Math|Random|RandomInteger 20)) "0, 0, 0" "1.000000,1.000000,1.000000" "KeepWorldPosition"))

(event Custom|Monster_OnDeadAnimationFinished
  (Utilities|FlowControl|Delay 5.0)
  (Actor|DestroyActor))

(event Custom|Monster_OnDead)

(event Custom|ResetApplyDamage
  ;[1 1 1] Player Damage
  (Variables|Default|SetCanApplyDamage? true)
  (Utilities|FlowControl|DoOnce false) ; enters at Reset
)

(event Custom|SetApplyDamage
  ;[1 1 1] Player Damage
  (Variables|Default|SetCanApplyDamage? true))

(event Custom|RagDollMulticast)

(event Custom|PlayAnimationMulticast
  (params (AnimMontage :type Anim%20Montage%20Object%20Reference))
  (Animation|PlayAnimMontage AnimMontage 1.0 "None"))

(event Custom|DisableAnimationMulticast
  (Class|AnimInstance|MontagePause (Components|SkeletalMesh|GetAnimInstance (Variables|Character|GetMesh)) (Animation|GetCurrentMontage :!class /Script/Engine.Character))
  (Components|Activation|Deactivate (Variables|Character|GetMesh)))

(event Custom|Monster_OnSight)

(event Custom|Monster_OnLoseSight)

(event Custom|Monster_OnInvestigateStart)

(event Custom|Monster_OnChaseStart)

(event EventBeginPlay
  (Transformation|AttachComponentToComponent (Variables|Default|GetHit%20Sphere) (Variables|Character|GetMesh) "hand_r" "KeepRelative" "KeepRelative" "KeepRelative" true)
  (Utilities|Time|SetTimerbyFunctionName 0 "MonsterBackgroundSound" 1.0 true))

(event Game|Damage|EventPointDamage
  (params (Damage :type Float%20%28single-precision%29) (DamageType :type Damage%20Type%20Object%20Reference) (HitLocation :type Vector :default "0, 0, 0") (HitNormal :type Vector :default "0, 0, 0") (HitComponent :type Primitive%20Component%20Object%20Reference) (BoneName :type Name :default "None") (ShotFromDirection :type Vector :default "0, 0, 0") (InstigatedBy :type Controller%20Object%20Reference) (DamageCauser :type Actor%20Object%20Reference) (HitInfo :type Hit%20Result%20Structure%20%28by%20ref%29))
  (bind (_dead _dyninganimationtime _die_) (CallFunction|MonsterGetDamage Damage DamageCauser))
  (if _dead
    (Utilities|FlowControl|Delay _dyninganimationtime)
    (CallFunction|MonsterFinishDeathAnimation _die_)))

(event Game|Damage|EventAnyDamage
  (params (Damage :type Float%20%28single-precision%29) (DamageType :type Damage%20Type%20Object%20Reference) (InstigatedBy :type Controller%20Object%20Reference) (DamageCauser :type Actor%20Object%20Reference))
  (bind (_dead _dyninganimationtime _die_) (CallFunction|MonsterGetDamage Damage DamageCauser))
  (if _dead
    (Utilities|FlowControl|Delay _dyninganimationtime)
    (CallFunction|MonsterFinishDeathAnimation _die_)
    (else
      (CallFunction|PlayEmitterMulticast))))

(fn ConstructionScript)

(fn MonsterGetDamage
  (params (Damage :type Float%20%28double-precision%29) (InstigatorActor :type Actor%20Object%20Reference))
  (Utilities|IsValid (AI|GetBlackboard 0)
    (:Is%20Valid
      (AI|Components|Blackboard|SetValueasEnum (AI|GetBlackboard 0) (Utilities|Name|MakeLiteralName "Status") (Utilities|Enum|LiteralenumMonsterStatus "NewEnumerator3"))
      (bind _health_after_damage (CallFunction|MonsterCalculateHealth Damage))
      (AI|Components|Blackboard|SetValueasVector (AI|GetBlackboard 0) (Utilities|Name|MakeLiteralName "DamageCauserLocation") (Transformation|GetActorLocation InstigatorActor))
      (CallFunction|MonsterCheckforFlee)
      (if (<= _health_after_damage 0.0)
        ;[1 1 1] 죽지않게 설정
        (Variables|Monster|SetIsUnbeatable true)
        (if (Utilities|IsValid (Pawn|GetController))
          _)))))

(fn MonsterCalculateHealth
  (params (Damage :type Float%20%28double-precision%29))
  (if (not (Variables|Monster|GetIsUnbeatable))
    (if (> (Variables|Monster|GetHealth) 0.0)
      (bind _output_get (Variables|Monster|SetHealth (- (Variables|Monster|GetHealth) Damage)))
      (return _output_get))))

(fn MonsterCheckforFlee
  (if (Math|Boolean|ANDBoolean (Variables|Monster|GetFlee?) (!= (Class|BlackboardComponent|GetValueasEnum (AI|GetBlackboard 0) (Utilities|Name|MakeLiteralName "Status")) (Utilities|Enum|LiteralenumMonsterStatus "NewEnumerator5")) (< (Variables|Monster|GetHealth) (Variables|Monster|GetFleeHealthTreshold)))
    (AI|Components|Blackboard|SetValueasEnum (AI|GetBlackboard 0) (Utilities|Name|MakeLiteralName "GeneralMode") (Utilities|Enum|LiteralenumMonsterGeneralMode "NewEnumerator1"))
    (AI|Components|Blackboard|SetValueasEnum (AI|GetBlackboard 0) (Utilities|Name|MakeLiteralName "Status") (Utilities|Enum|LiteralenumMonsterStatus "NewEnumerator5"))
    (Variables|/Script/Engine.CharacterMovementComponent|SetMaxWalkSpeed (Variables|Character|GetCharacterMovement) (Variables|MonsterValues|GetMaxSpeed))))

(fn MonsterFinishDeathAnimation
  (params (Die? :type Boolean))
  (if (not Die?)
    (CallFunction|DisableAnimationMulticast)))

(fn MonsterPerception
  (params (Actor :type Actor%20Object%20Reference) (Stimulus :type AI%20Stimulus%20Structure))
  (bind _bsuccessfullysensed (Utilities|Struct|BreakAIStimulus Stimulus))
  (bind _returnvalue (AI|GetBlackboard 0))
  (bind _returnvalue_2 (AI|GetBlackboard 0))
  (bind _returnvalue_3 (Class|AIPerceptionSystem|GetSenseClassforStimulus Stimulus))
  (if (== _returnvalue_3 "/Script/AIModule.AISense_Sight")
    (if (or (== Actor (Game|GetPlayerCharacter 0)) (Actor|ActorHasTag Actor "player"))
      (Utilities|IsValid _returnvalue_2
        (:Is%20Valid
          (AI|Components|Blackboard|SetValueasObject _returnvalue_2 (Utilities|Name|MakeLiteralName "TargetActor") Actor)
          (AI|Components|Blackboard|SetValueasBool (AI|GetBlackboard 0) (Utilities|Name|MakeLiteralName "CanSeePlayer?") _bsuccessfullysensed)
          (Utilities|FlowControl|Sequence
            (:then_0
              (if _bsuccessfullysensed
                (AI|Components|Blackboard|SetValueasEnum (AI|GetBlackboard 0) (Utilities|Name|MakeLiteralName "Status") (Utilities|Enum|LiteralenumMonsterStatus "NewEnumerator4"))
                (CallFunction|MonsteronSight)
                (else
                  (AI|Components|Blackboard|SetValueasEnum (AI|GetBlackboard 0) (Utilities|Name|MakeLiteralName "Status") (Utilities|Enum|LiteralenumMonsterStatus "NewEnumerator2"))
                  (CallFunction|MonsteronChaseStart))))
            (:then_1
              (if (not _bsuccessfullysensed)
                (CallFunction|MonsteronLoseSight)))))))
    (elif true
      (if (not (ScalableFloat|GetValueasBool (AI|GetBlackboard 0) (Utilities|Name|MakeLiteralName "CanSeePlayer?")))
        (AI|Components|Blackboard|SetValueasObject _returnvalue (Utilities|Name|MakeLiteralName "TargetActor") 0)
        (AI|Components|Blackboard|SetValueasVector _returnvalue (Utilities|Name|MakeLiteralName "TargetLocation") (Transformation|GetActorLocation Actor))
        (if (== (Class|BlackboardComponent|GetValueasEnum (AI|GetBlackboard 0) (Utilities|Name|MakeLiteralName "Status")) (Utilities|Enum|LiteralenumMonsterStatus "NewEnumerator1"))
          ;[1 1 1] Nothing으로 설정해서 소리를 들을 때 마다 재설정 가능
          (if (Variables|Default|GetCanSearch?)
            (AI|Components|Blackboard|SetValueasEnum (AI|GetBlackboard 0) (Utilities|Name|MakeLiteralName "Status") (Utilities|Enum|LiteralenumMonsterStatus "NewEnumerator6"))
            (AI|Components|Blackboard|SetValueasEnum (AI|GetBlackboard 0) (Utilities|Name|MakeLiteralName "Status") (Utilities|Enum|LiteralenumMonsterStatus "NewEnumerator1") :!label _label)
            (Variables|Default|SetCanSearch? false)
            (CallFunction|ResetHearing)
            (CallFunction|MonsteronHearing))
          (elif (Variables|Default|GetCanSearch?)
            (goto _label)))))))

(fn MonsterBackgroundSound
  (Audio|PlaySoundatLocation "/Game/BG/BP/Sound/Moster_Water.Moster_Water" (Transformation|GetActorLocation) "0, 0, 0" 1.0 1.0 0.0 0 0 0 0))